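; BP_Pawn is a pawn moved by the Enhanced Input action IA_Move, with a start position that follows the player's progress.
; Move input becomes a swept, frame-rate-independent local offset scaled by Velocidad, which is set on BeginPlay.
; Every Tick it reads PartesPasadas (parts passed) from BP_MyPlayerController and picks one of three hard-coded PosicionInicial vectors.
; This Blueprint only stores that position and never applies it.
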(event `self.ReceiveTick`
  (params (DeltaSeconds :type "Float (single-precision)"))
  (bind _asbp_my_player_controller (cast `/Game/Framework/BP_MyPlayerController` (`GameplayStatics.GetPlayerController` 0)))
  (bind _partespasadas (`/Game/Framework/BP_MyPlayerController.PartesPasadas` _asbp_my_player_controller))
  (`/Engine/EditorBlueprintResources/StandardMacros.CompareInt` _partespasadas
    (:`>`
      (`/Engine/EditorBlueprintResources/StandardMacros.CompareInt` _partespasadas 1
        (:`>`
          (set `self.PosicionInicial` (`KismetMathLibrary.MakeVector` 2120.0 -5460.0)))
        (:`==`
          (set `self.PosicionInicial` (`KismetMathLibrary.MakeVector` 5370.0 -5760.0)))))
    (:`==`
      (set `self.PosicionInicial` (`KismetMathLibrary.MakeVector` 1.0)))))

(event `self.ReceiveBeginPlay`
  (set `self.Velocidad` 1.0))

(event `EnhancedInput|/Game/Framework/IA_Move`
  (params (ActionValue :type "Vector2D Structure") (ElapsedSeconds :type "Float (double-precision)") (TriggeredSeconds :type "Float (double-precision)") (InputAction :type "InputAction Object Reference" :default "/Game/Framework/IA_Move.IA_Move"))
  (:`Triggered`
    (`self.K2_AddActorLocalOffset` (* (`KismetMathLibrary.Conv_Vector2DToVector` ActionValue) (900.0 900.0 900.0) (`self.Velocidad`) (`GameplayStatics.GetWorldDeltaSeconds`)) true)))

(fn `UserConstructionScript`)