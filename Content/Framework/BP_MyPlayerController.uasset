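; BP_MyPlayerController is a player controller that sets up Enhanced Input and keeps the player's score.
; On BeginPlay it adds the BP_MyInputMappingContext mapping context and resets the Puntos, PartesPasadas and Muertes counters.
; IncrementScore_Event increments Puntos, then finds the first top-level WBP_Score widget by class search and writes the new value directly into its text block.
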(event `self.ReceiveBeginPlay`
  (`EnhancedInputSubsystemInterface.AddMappingContext` (subsystem `EnhancedInputLocalPlayerSubsystem`) "/Game/Framework/BP_MyInputMappingContext.BP_MyInputMappingContext" 0 (struct))
  (set `self.Puntos` 0)
  (set `self.PartesPasadas` 0)
  (set `self.Muertes` 0))

(event `self.ReceiveTick`
  (params (DeltaSeconds :type "Float (single-precision)")))

(event `IncrementScore_Event`
  (bind _result (`/Engine/EditorBlueprintResources/StandardMacros.IncrementInt` (`self.Puntos`))
    (:`  `
      (set `self.Puntos` _result)
      (bind _foundwidgets (`WidgetBlueprintLibrary.GetAllWidgetsOfClass` "/Game/BPs/WBP_Score.WBP_Score_C"))
      (bind _output_get (set `self.WidgetScore` (`|GetArrayItem` _foundwidgets)))
      (`TextBlock.SetText` (`/Game/BPs/WBP_Score.TextBlock_28` _output_get) (`KismetTextLibrary.Conv_IntToText` (`self.Puntos`))))))

(fn `UserConstructionScript`)